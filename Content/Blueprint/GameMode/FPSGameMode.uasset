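; Game mode for an FPS drone-clearing round, won by killing every drone before time runs out while staying alive.
; Tick switches on a session state: warmup with input disabled, timed play, then win, death or timeout.
; DroneDied counts down the drones found at BeginPlay, while a HUD widget shows count, timer and announcements.
; End states disable input and run a delay-loop countdown macro before reloading the level.
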(event EventBeginPlay
  (Utilities|FlowControl|Sequence
    (:then_0
      ;[1 1 1] Add Gamemode HUD
      (bind _returnvalue (UserInterface|CreateWidget "/Game/Blueprint/HUD/GameModeHUD.GameModeHUD_C"))
      (bind _output_get (Variables|Default|SetGameModeHUD _returnvalue))
      (UserInterface|Viewport|AddtoViewport _output_get 0)
      (Rendering|Components|TextRender|SetText (Variables|/Game/Blueprint/HUD/GameModeHUD.GameModeHUD_C|GetAnnouncement _output_get) "Clear the Zone!")
      (bind _format_time (CallFunction|TimeRemainingFormat))
      (Rendering|Components|TextRender|SetText (Variables|/Game/Blueprint/HUD/GameModeHUD.GameModeHUD_C|GetTimeText _output_get) _format_time))
    (:then_1
      ;[1 1 1] Set Number of Drones
      (bind _outactors (Actor|GetAllActorsOfClass "/Game/Blueprint/Drone/Drone_Pawn.Drone_Pawn_C"))
      (bind _output_get_2 (Variables|Default|SetNumberOfDrones (Utilities|Array|Length _outactors)))
      (Rendering|Components|TextRender|SetText (Variables|/Game/Blueprint/HUD/GameModeHUD.GameModeHUD_C|GetDroneNumber (Variables|Default|GetGameModeHUD)) (Utilities|Text|ToText(Integer) _output_get_2)))
    (:then_2
      ;[1 1 1] Disable Player Input on Warmup
      (CallFunction|DisablePlayerInput))))

(event EventTick
  (params (DeltaSeconds :type Float%20%28single-precision%29))
  (switch Utilities|FlowControl|Switch|SwitchonSessionState (Variables|Default|GetSessionState)
    (:NewEnumerator0
      (CallFunction|UpdateWarmupTimer))
    (:NewEnumerator1
      (CallFunction|UpdateGameTimer DeltaSeconds))
    (:NewEnumerator2
      (Utilities|Coutndown :!label _label)
      (CallFunction|ResetLevel))
    (:NewEnumerator3
      (goto _label))
    (:NewEnumerator4
      (goto _label))))

(fn ConstructionScript)

(fn DroneDied
  ;[1 1 1] Checks if Player is Alive
  (bind _asfps_character (Utilities|Casting|CastToFPS_Character (Game|Player|GetPlayerPawn 0)))
  (if (> (Variables|/Game/Blueprint/Character/FPS_Character.FPS_Character_C|GetHealth _asfps_character) 0.0)
    (bind _result (Math|Integer|DecrementInt (Variables|Default|GetNumberOfDrones))
      (:%20%20
        (Rendering|Components|TextRender|SetText (Variables|/Game/Blueprint/HUD/GameModeHUD.GameModeHUD_C|GetDroneNumber (Variables|Default|GetGameModeHUD)) (Utilities|Text|ToText(Integer) _result))
        (if (<= (Variables|Default|GetNumberOfDrones) 0)
          (CallFunction|PlayerWon))))))

(fn UpdateWarmupTimer
  (bind _returnvalue (Utilities|Time|GetGameTimeinSeconds))
  (bind _warmuptime (Variables|Default|GetWarmupTime))
  (bind _returnvalue_2 (- _warmuptime _returnvalue))
  (Rendering|Components|TextRender|SetText (Variables|/Game/Blueprint/HUD/GameModeHUD.GameModeHUD_C|GetWarmupText (Variables|Default|GetGameModeHUD)) (Utilities|Text|ToText(Float) _returnvalue_2 "HalfToEven" false true 1 324 0 0))
  (if (<= _returnvalue_2 0.0)
    (CallFunction|StartGame)))

(fn EnablePlayerInput
  (bind _returnvalue (Game|Player|GetPlayerPawn 0))
  (bind _asfps_character (Utilities|Casting|CastToFPS_Character _returnvalue))
  (Variables|/Game/Blueprint/Character/FPS_Character.FPS_Character_C|SetFireButtonPressed _asfps_character true)
  (Input|EnableInput _returnvalue 0))

(fn DisablePlayerInput
  (bind _returnvalue (Game|Player|GetPlayerPawn 0))
  (bind _asfps_character (Utilities|Casting|CastToFPS_Character _returnvalue))
  (Variables|/Game/Blueprint/Character/FPS_Character.FPS_Character_C|SetFireButtonPressed _asfps_character false)
  (Input|DisableInput _returnvalue 0))

(fn StartGame
  (bind _gamemodehud (Variables|Default|GetGameModeHUD))
  (Variables|Default|SetSessionState "NewEnumerator1")
  (CallFunction|EnablePlayerInput)
  (Rendering|Components|TextRender|SetText (Variables|/Game/Blueprint/HUD/GameModeHUD.GameModeHUD_C|GetWarmupText _gamemodehud) "")
  (Rendering|Components|TextRender|SetText (Variables|/Game/Blueprint/HUD/GameModeHUD.GameModeHUD_C|GetAnnouncement _gamemodehud) ""))

(fn UpdateGameTimer
  (params (Delta%20Time :type Float%20%28double-precision%29))
  (bind _gamemodehud (Variables|Default|GetGameModeHUD))
  (bind _timetext (Variables|/Game/Blueprint/HUD/GameModeHUD.GameModeHUD_C|GetTimeText _gamemodehud))
  (Variables|Default|SetTimeRemaining (- (Variables|Default|GetTimeRemaining) Delta%20Time))
  ;[1 1 1] Converts Time into 00:00 Format
  (bind _format_time (CallFunction|TimeRemainingFormat))
  (Rendering|Components|TextRender|SetText _timetext _format_time)
  ;[1 1 1] If Timer is <= 00:10, Timer text turns Red.
  (if (<= (Variables|Default|GetTimeRemaining) 1e+01)
    (Appearance|SetColorandOpacity _timetext (Utilities|Struct|MakeSlateColor "(R=1.000000,G=0.000000,B=0.023098,A=1.000000)") :!class /Script/UMG.TextBlock)
    ;[1 1 1] If Timer is <= 00:00, Play Out of Time.
    (if (<= (Variables|Default|GetTimeRemaining) 0.0)
      (CallFunction|OutOfTime))))

(fn OutOfTime
  (bind _gamemodehud (Variables|Default|GetGameModeHUD))
  (Variables|Default|SetSessionState "NewEnumerator2")
  (CallFunction|DisablePlayerInput)
  (Rendering|Components|TextRender|SetText (Variables|/Game/Blueprint/HUD/GameModeHUD.GameModeHUD_C|GetTimeText _gamemodehud) "00:00")
  (Rendering|Components|TextRender|SetText (Variables|/Game/Blueprint/HUD/GameModeHUD.GameModeHUD_C|GetAnnouncement _gamemodehud) "Out of Time! Resetting Level in:"))

(fn TimeRemainingFormat
  (bind _timeremaining (Variables|Default|GetTimeRemaining))
  (bind _returnvalue (/ _timeremaining 6e+01))
  (bind _returnvalue_2 (Class|KismetMathLibrary|FFloor64 _returnvalue))
  (return (Utilities|Text|FormatText "{Minutes}:{Seconds}" (Utilities|Text|ToText(String) _returnvalue_2) (Utilities|Text|ToText(String) (- (Variables|Default|GetTimeRemaining) (* _returnvalue_2 6e+01)) false true 2 2))))

(fn PlayerWon
  (Variables|Default|SetSessionState "NewEnumerator4")
  (Rendering|Components|TextRender|SetText (Variables|/Game/Blueprint/HUD/GameModeHUD.GameModeHUD_C|GetAnnouncement (Variables|Default|GetGameModeHUD)) "You Win! Resetting Level in:")
  (CallFunction|DisablePlayerInput))

(fn PlayerDied
  (bind _gamemodehud (Variables|Default|GetGameModeHUD))
  (Variables|Default|SetSessionState "NewEnumerator3")
  (Rendering|Components|TextRender|SetText (Variables|/Game/Blueprint/HUD/GameModeHUD.GameModeHUD_C|GetAnnouncement _gamemodehud) "You Died! Resetting Level in:")
  (Rendering|Components|TextRender|SetText (Variables|/Game/Blueprint/HUD/GameModeHUD.GameModeHUD_C|GetTimeText _gamemodehud) "00:00")
  (CallFunction|DisablePlayerInput))

(fn ResetLevel
  (bind _returnvalue (Game|GetCurrentLevelName true))
  (Game|OpenLevel(byName) (Utilities|String|StringToName _returnvalue)))